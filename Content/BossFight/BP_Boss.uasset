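; Boss enemy Blueprint that tracks health and shows it on an on-screen health bar.
; BeginPlay creates the WB_BossHP widget, and Tick sets its bar percent from Health against a hardcoded maximum.
; AnyDamage subtracts from Health and, at zero or below, disables movement and turns on mesh physics simulation for a ragdoll death.
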(event EventBeginPlay
  (bind _returnvalue (Game|ConstructObjectfromClass "/Game/BossFight/WB_BossHP.WB_BossHP_C"))
  (UserInterface|Viewport|AddtoViewport _returnvalue 0)
  (Variables|Default|SetHPUI _returnvalue))

(event Collision|EventActorBeginOverlap
  (params (OtherActor :type Actor%20Object%20Reference)))

(event EventTick
  (params (DeltaSeconds :type Float%20%28single-precision%29))
  (Progress|SetPercent (Variables|/Game/BossFight/WB_BossHP.WB_BossHP_C|GetHealthBar (Variables|Default|GetHPUI)) (/ (Variables|Default|GetHealth) 1e+03)))

(event Game|Damage|EventAnyDamage
  (params (Damage :type Float%20%28single-precision%29) (DamageType :type Damage%20Type%20Object%20Reference) (InstigatedBy :type Controller%20Object%20Reference) (DamageCauser :type Actor%20Object%20Reference))
  (Variables|Default|SetHealth (- (Variables|Default|GetHealth) Damage))
  (if (<= (Variables|Default|GetHealth) 0.0)
    (Pawn|Components|CharacterMovement|DisableMovement (Variables|Character|GetCharacterMovement))
    (Physics|SetSimulatePhysics (Variables|Character|GetMesh) true)))

(fn ConstructionScript)