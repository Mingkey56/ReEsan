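; BP_BIS_Path is a spline path actor that marks its route with direction decals, built in the construction script.
; For every spline point except the last, it adds a downward-pitched decal, placed and yawed via lerp and look-at on local point locations.
; Vector length and height difference drive the decal scale.
; Each decal gets its own M_BIS_Direction dynamic material, whose Size parameter matches the length-based scale.
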(fn ConstructionScript
  (bind _spline (Variables|Default|GetSpline))
  (bind _returnvalue (Spline|GetNumberOfSplinePoints _spline))
  (for _index (range 0 _returnvalue)
    (if (< _index (- _returnvalue 1))
      (bind _returnvalue_2 (Rendering|Material|CreateDynamicMaterialInstance "/Game/Basic_Interaction_System/Materials/M_BIS_Direction.M_BIS_Direction" "None" "None" :!class /Script/Engine.KismetMaterialLibrary))
      (Rendering|Material|SetScalarParameterValue _returnvalue_2 "Size" (/ (- (Math|Vector|VectorLength (Spline|GetLocationatSplinePoint (Variables|Default|GetSpline) _index "Local")) 2e+02) 2e+02) :!class /Script/Engine.MaterialInstanceDynamic)
      (bind _returnvalue_3 (AddComponent|AddDecalComponent false (Math|Transform|MakeTransform (Math|Vector|Lerp(Vector) (Spline|GetLocationatSplinePoint (Variables|Default|GetSpline) _index "Local") (Spline|GetLocationatSplinePoint (Variables|Default|GetSpline) _index "Local") 0.5) (Math|Rotator|MakeRotator 0.0 9e+01 (+ (.yaw (Math|Rotator|FindLookatRotation (Spline|GetLocationatSplinePoint (Variables|Default|GetSpline) _index "Local") (Spline|GetLocationatSplinePoint (Variables|Default|GetSpline) _index "Local"))) -9e+01)) (Math|Vector|MakeVector (+ (/ (Math|Float|Absolute(Float) (.Z (Math|Vector|BreakVector (- (Math|Vector|Lerp(Vector) (Spline|GetLocationatSplinePoint (Variables|Default|GetSpline) _index "Local") (Spline|GetLocationatSplinePoint (Variables|Default|GetSpline) _index "Local") 0.5) (Spline|GetLocationatSplinePoint (Variables|Default|GetSpline) _index "Local"))))) 2e+02) 0.5) (/ (- (Math|Vector|VectorLength (Spline|GetLocationatSplinePoint (Variables|Default|GetSpline) _index "Local")) 2e+02) 2e+02) 0.1))))
      (Rendering|Components|Decal|SetDecalMaterial _returnvalue_3 _returnvalue_2))))