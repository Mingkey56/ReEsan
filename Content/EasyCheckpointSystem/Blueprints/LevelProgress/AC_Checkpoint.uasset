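; Actor component that respawns its owning character at a stored transform, which defaults to the owner's transform at BeginPlay.
; Respawn gets the player character from the owner through a message call, ragdolls it, then restores it after a short delay.
; Recovery teleports the character, reattaches the mesh to the capsule at its cached relative transform, and restores collision and walking.
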(event Custom|Event%20Respawn
  ;[0.15 0.15 0.15 0.5] Respawn entry point: triggers a short ragdoll phase on the player, then after a delay restores control and teleports the character back to the stored checkpoint transform.
  (bind _character (Class|BPIGetPlayerCharacter|GetPlayerCharacter(Message) (Components|GetOwner)))
  (CallFunction|RagdollStart _character)
  (Utilities|FlowControl|Delay 2.0)
  (Physics|SetSimulatePhysics (Variables|/Script/Engine.Character|GetMesh _character) false)
  (Utilities|FlowControl|Delay 0.01)
  (CallFunction|RagdollEnd _character))

(event EventBeginPlay
  (bind _returnvalue (Components|GetOwner))
  ;[0.149 0.149 0.149 0.502] Initializes the respawn data for the owning character: stores the owner's starting world transform as the default respawn point and caches the Skeletal Mesh's relative transform so its position and rotation can be restored correctly after ragdoll.
  (Variables|Default|SetRespawnActorTransform (Transformation|GetActorTransform _returnvalue))
  (Variables|Default|SetDefaultMeshRelativeTransform (Transformation|GetRelativeTransform (Actor|GetComponentbyClass _returnvalue "/Script/Engine.SkeletalMeshComponent"))))

(fn RagdollStart
  (params (Character :type Character%20Object%20Reference))
  (bind _mesh (Variables|/Script/Engine.Character|GetMesh Character))
  ;[0.15 0.15 0.15 0.5] Switches the character into ragdoll: temporarily disables standard locomotion/control, adjusts collision setup, and enables physics simulation on the Skeletal Mesh. Also caches the required transforms to restore a clean pose/position after ragdoll.
  (Pawn|Components|CharacterMovement|SetMovementMode (Variables|/Script/Engine.Character|GetCharacterMovement Character) "MOVE_None" 0)
  (Collision|SetCollisionEnabled (Variables|/Script/Engine.Character|GetCapsuleComponent Character) "NoCollision")
  (Collision|SetCollisionProfileName _mesh "Ragdoll" true :!class /Script/Engine.PrimitiveComponent)
  (Physics|SetSimulatePhysics _mesh true))

(fn RagdollEnd
  (params (Character :type Character%20Object%20Reference))
  (bind _mesh (Variables|/Script/Engine.Character|GetMesh Character))
  (bind _capsulecomponent (Variables|/Script/Engine.Character|GetCapsuleComponent Character))
  (bind _respawnactortransform (Variables|Default|GetRespawnActorTransform))
  ;[0.15 0.15 0.15 0.5] Exits ragdoll and returns to normal gameplay: sets movement mode back to Walking, restores collisions, disables Mesh physics simulation, and snaps the character back to the cached transforms (mesh relative transform + actor location/rotation) using Teleport to prevent jitter and leftover physics momentum.
  (Transformation|SetActorLocationAndRotation Character (.location _respawnactortransform) (.rotation _respawnactortransform) false true)
  (Transformation|AttachComponentToComponent _mesh _capsulecomponent "None" "SnapToTarget" "SnapToTarget" "KeepRelative" false)
  (Transformation|SetRelativeTransform _mesh (Variables|Default|GetDefaultMeshRelativeTransform) false true)
  (Collision|SetCollisionProfileName _mesh "CharacterMesh" true :!class /Script/Engine.PrimitiveComponent)
  (Collision|SetCollisionEnabled _capsulecomponent "QueryAndPhysics")
  (Pawn|Components|CharacterMovement|SetMovementMode (Variables|/Script/Engine.Character|GetCharacterMovement Character) "MOVE_Walking" 0))