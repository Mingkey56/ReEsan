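; BP_Tailsman is a talisman weapon actor that stuns enemies and can be picked up by the player.
; When Box overlaps a BP_Enemy, it stuns the enemy, attaches its static mesh to the enemy's mesh, then destroys itself after a delay.
; When Box1 overlaps the first-person character, it hides the character's HTailsman component, grants and selects the talisman weapon slot, then destroys itself.
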(event OnComponentBeginOverlap(Box)
  (params (OverlappedComponent :type Primitive%20Component%20Object%20Reference) (OtherActor :type Actor%20Object%20Reference) (OtherComp :type Primitive%20Component%20Object%20Reference) (OtherBodyIndex :type Integer) (bFromSweep :type Boolean) (SweepResult :type Hit%20Result%20Structure%20%28by%20ref%29))
  (bind _asbp_enemy (Utilities|Casting|CastToBP_Enemy OtherActor))
  (Default|IsStunned _asbp_enemy 4.0)
  (Transformation|AttachComponentToComponent (Variables|Default|GetStaticMesh) (Variables|/Script/Engine.Character|GetMesh _asbp_enemy) "None" "KeepRelative" "KeepRelative" "KeepRelative" true)
  (Utilities|FlowControl|Delay 5.0)
  (Actor|DestroyActor))

(event OnComponentBeginOverlap(Box1)
  (params (OverlappedComponent :type Primitive%20Component%20Object%20Reference) (OtherActor :type Actor%20Object%20Reference) (OtherComp :type Primitive%20Component%20Object%20Reference) (OtherBodyIndex :type Integer) (bFromSweep :type Boolean) (SweepResult :type Hit%20Result%20Structure%20%28by%20ref%29))
  (bind _asbp_first_person_character_me (Utilities|Casting|CastToBP_FirstPersonCharacterME OtherActor))
  (Rendering|SetVisibility (Variables|/Game/FirstPerson/Blueprints/BP_FirstPersonCharacterME.BP_FirstPersonCharacterME_C|GetHTailsman _asbp_first_person_character_me) false false)
  (Variables|/Game/FirstPerson/Blueprints/BP_FirstPersonCharacterME.BP_FirstPersonCharacterME_C|SetbHasTailsman _asbp_first_person_character_me true)
  (Variables|/Game/FirstPerson/Blueprints/BP_FirstPersonCharacterME.BP_FirstPersonCharacterME_C|SetCurrentWeapon _asbp_first_person_character_me 4)
  (Actor|DestroyActor))

(event EventBeginPlay)

(event Collision|EventActorBeginOverlap
  (params (OtherActor :type Actor%20Object%20Reference)))

(event EventTick
  (params (DeltaSeconds :type Float%20%28single-precision%29)))

(fn ConstructionScript)