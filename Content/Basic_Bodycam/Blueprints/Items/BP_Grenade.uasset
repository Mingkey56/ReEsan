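; BP_Grenade is a timed grenade actor that explodes and deals radial damage shortly after spawning.
; On BeginPlay it waits out a fixed fuse, spawns explosion particles and sound at its Sphere, applies radial damage from its damage and radius variables, then destroys itself.
; Sphere hits play a metal clink, throttled by a DoOnce that resets after a short delay to avoid rapid repeats.
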(event OnComponentHit(Sphere)
  (params (HitComponent :type Primitive%20Component%20Object%20Reference) (OtherActor :type Actor%20Object%20Reference) (OtherComp :type Primitive%20Component%20Object%20Reference) (NormalImpulse :type Vector :default "0, 0, 0") (Hit :type Hit%20Result%20Structure%20%28by%20ref%29))
  ;[0.15 0.15 0.15 0.5] Making the Impact Sounds
  (Utilities|FlowControl|DoOnce false :!label _label
    (:Completed
      (Audio|PlaySoundatLocation "/Game/Basic_Bodycam/Sounds/SW_Metal_Clink.SW_Metal_Clink" (Transformation|GetWorldLocation (Variables|Default|GetSphere)) "0, 0, 0" 1.0 1.0 0.0 "/Game/Basic_Bodycam/Sounds/SA_Gunshot.SA_Gunshot" 0 0 0)
      (Utilities|FlowControl|Delay 0.1) ; Adding a small delay between sounds so the don't repeat too quickly
      (goto _label Reset))))

(event EventBeginPlay
  ;[0.15 0.15 0.15 0.5] Spawning the effects and dealing damage
  (Utilities|FlowControl|Delay 3.0) ; Waiting 3 seconds before the explosion
  (Effects|SpawnEmitteratLocation "/Game/Basic_Bodycam/Demo/Particles/P_Explosion.P_Explosion" (Transformation|GetWorldLocation (Variables|Default|GetSphere)) "0, 0, 0" "2.000000,2.000000,2.000000")
  (Audio|SpawnSoundatLocation "/Game/Basic_Bodycam/Demo/Audio/Explosion01.Explosion01" (Transformation|GetWorldLocation (Variables|Default|GetSphere)) "0, 0, 0" 1.3 1.0 0.0 "/Game/Basic_Bodycam/Sounds/SA_Gunshot.SA_Gunshot" 0)
  (Game|Damage|ApplyRadialDamage (Variables|Default|GetgrenadeDamage) (Transformation|GetWorldLocation (Variables|Default|GetSphere)) (Variables|Default|GetgrenadeRadius) 0 0 0 0 false "ECC_Visibility") ; Dealing damage based on distance
  (Actor|DestroyActor))

(fn ConstructionScript)