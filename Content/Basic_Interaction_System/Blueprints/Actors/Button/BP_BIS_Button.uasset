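; BP_BIS_Button is an interactable button in the Basic Interaction System that toggles the lights in the level.
; On an Activate interaction status, a FlipFlop alternates between pressed and released, nudging the button along X and choosing on or off light intensity and material.
; It then finds every BP_BIS_Light actor and applies that material to its cylinder and intensity to its point light.
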(event EventUpdateInteract
  (params (Actor :type Actor%20Object%20Reference) (Status :type E_BIS_ItemType%20Enum :default "NewEnumerator0") (Widget :type WBP%20BIS%20Inventory%20Object%20Reference))
  ;[0.4118 0.9216 1] Event Update Interact
  (switch Utilities|FlowControl|Switch|SwitchonE_BIS_ItemType Status
    (:NewEnumerator6
      (Utilities|FlowControl|FlipFlop
        (:A
          (Variables|Default|SetDelta%20Location%20X -5.0)
          (Variables|Default|SetLight%20Intensity 5e+01)
          (Variables|Default|SetLight%20Material "/Game/Basic_Interaction_System/Materials/M_lightsOn.M_lightsOn"))
        (:B
          (Variables|Default|SetDelta%20Location%20X 5.0)
          (Variables|Default|SetLight%20Intensity 0.0)
          (Variables|Default|SetLight%20Material "/Game/Basic_Interaction_System/Materials/M_lightsOff.M_lightsOff")))
      (Transformation|AddRelativeLocation (Variables|Default|GetDefaultSceneRoot) (Math|Vector|MakeVector (Variables|Default|GetDelta%20Location%20X) 0.0 0.0) false true)
      (bind _outactors (Actor|GetAllActorsOfClass "/Game/Basic_Interaction_System/Blueprints/Actors/Lights/BP_BIS_Light.BP_BIS_Light_C"))
      (for _array_element _outactors
        (Rendering|Material|SetMaterial (Variables|/Game/Basic_Interaction_System/Blueprints/Actors/Lights/BP_BIS_Light.BP_BIS_Light_C|GetCylinder _array_element) 0 (Variables|Default|GetLight%20Material))
        (Rendering|Components|Light|SetIntensity (Variables|/Game/Basic_Interaction_System/Blueprints/Actors/Lights/BP_BIS_Light.BP_BIS_Light_C|GetPointLight _array_element) (Variables|Default|GetLight%20Intensity))))))

(fn ConstructionScript)