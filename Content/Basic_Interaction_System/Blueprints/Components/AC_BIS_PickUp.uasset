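; Actor component that lets its owning item be picked up and set down by the first-person character in the interaction system.
; Pick Up saves the item's rotation, attaches it to the mesh's GripPoint socket, sets HasKey on the anim blueprint and updates the interact message.
; Throw traces from the camera and, only on actors tagged Ground, detaches and teleports the item to the hit point with its saved rotation.
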(event Custom|Event%20Pick%20Up
  (bind _returnvalue (Components|GetOwner))
  ;[0.4118 0.9216 1] Event Pick Up (item)
  (Variables|Default|SetStart%20Rotation (Transformation|GetActorRotation _returnvalue))
  (Transformation|SetActorRelativeRotation _returnvalue "0.000000,0.000000,90.000000" false true)
  (bind _asbp_bis_first_person_character (Utilities|Casting|CastToBP_BIS_FirstPersonCharacter (Variables|Default|GetActor)))
  (bind _output_get (Variables|Default|SetCharacter _asbp_bis_first_person_character))
  (Transformation|AttachComponentToComponent (Variables|/Script/Engine.Actor|GetRootComponent (Components|GetOwner)) (Variables|/Game/Basic_Interaction_System/Demo/FirstPerson/Blueprints/BP_BIS_FirstPersonCharacter.BP_BIS_FirstPersonCharacter_C|GetFirstPersonMesh _output_get) "GripPoint" "SnapToTarget" "SnapToTarget" "SnapToTarget" true)
  (bind _asfp_bis_anim_bp (Utilities|Casting|CastToFP_BIS_AnimBP (Components|SkeletalMesh|GetAnimInstance (Variables|/Game/Basic_Interaction_System/Demo/FirstPerson/Blueprints/BP_BIS_FirstPersonCharacter.BP_BIS_FirstPersonCharacter_C|GetFirstPersonMesh (Variables|Default|GetCharacter)))))
  (Variables|/Game/Basic_Interaction_System/Demo/FirstPersonArms/Animations/FP_BIS_AnimBP.FP_BIS_AnimBP_C|SetHasKey _asfp_bis_anim_bp true)
  (Class|BPIBISInteract|UpdateInteract(Message) (Variables|Default|GetActor) 0 "NewEnumerator0"))

(event Custom|Event%20Interaction
  (params (Actor :type Actor%20Object%20Reference) (Pick%20Up :type E_BIS_ItemType%20Enum :default "NewEnumerator0"))
  ;[0.4118 0.9216 1] Event Interaction
  (Variables|Default|SetActor Actor)
  (switch Utilities|FlowControl|Switch|SwitchonE_BIS_ItemType Pick%20Up
    (:NewEnumerator0
      (CallFunction|EventPickUp))
    (:NewEnumerator1
      (CallFunction|EventThrow))))

(event Custom|Event%20Throw
  (bind (_returnvalue _returnvalue2) (CallFunction|CameraVectors))
  ;[0.4118 0.9216 1] Event Throw (Item)
  (bind _outhit (Collision|LineTraceByChannel _returnvalue _returnvalue2 "TraceTypeQuery1" false 0 "None"))
  (Variables|Default|SetOut%20Hit%20Location (.location _outhit))
  (if (!= (Utilities|Array|FindItem (Variables|/Script/Engine.Actor|GetTags (.hitactor _outhit)) "Ground") -1)
    (Transformation|DetachFromActor (Components|GetOwner) "KeepWorld" "KeepWorld" "KeepWorld")
    (bind _returnvalue_2 (Transformation|SetActorLocationAndRotation (Components|GetOwner) (Variables|Default|GetOut%20Hit%20Location) (Variables|Default|GetStart%20Rotation) false true))
    (if _returnvalue_2
      (Class|BPIBISInteract|UpdateInteract(Message) (Variables|Default|GetActor) 0 "NewEnumerator2"))))

(fn CameraVectors
  (bind _returnvalue (Game|GetPlayerCameraManager 0))
  (bind _returnvalue_2 (Transformation|GetActorLocation _returnvalue))
  (return _returnvalue_2 (+ _returnvalue_2 (* (Math|Vector|GetForwardVector (Variables|/Script/Engine.Actor|GetRootComponent _returnvalue)) 5e+02))))