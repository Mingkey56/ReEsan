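; Game Instance that runs dialogue conversations, loading lines from a Data Table and showing them in a WBP_Subtitles widget.
; Each line sets speaker, text and prompt, then timers handle its duration and post-line delay before advancing.
; Normal lines auto-advance, Input lines wait for a continue call, and Event lines notify all BPI_DialogueEvents actors.
; A state enum tracks playback, and the widget collapses when the rows run out.
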(event Custom|EV_ShowCurrentDialogue
  (params (Speaker :type Name) (Dialogue :type Text) (Duration :type Float%20%28double-precision%29) (PromptText :type Text))
  (Utilities|IsValid (Variables|Default|GetDialogue_SubtitleWidget)
    (:Is%20Valid
      (Default|UpdateDialogue (Variables|Default|GetDialogue_CurrentWidget) Speaker Dialogue PromptText)
      (if (> Duration 0.0)
        (bind _returnvalue (Utilities|Time|SetTimerbyEvent (delegate Custom|EV_TimerFinished) Duration))
        (Variables|Default|SetDialogue_TimerDelay _returnvalue)
        (else
          (Variables|Default|SetDialogue_DelayTimeFinished true)
          (switch Utilities|FlowControl|Switch|SwitchonE_DialogueType (Variables|Default|GetDialogue_CurrentLineType)
            (:NewEnumerator0
              (CallFunction|EVDialogueCheckContinue :!label _label))
            (:NewEnumerator4
              (Variables|Default|SetDialogue_State "NewEnumerator2"))
            (:NewEnumerator2
              (bind _outactors (Actor|GetAllActorswithInterface "/Game/DialogueSystem/Blueprints/Interfaces/BPI_DialogueEvents.BPI_DialogueEvents_C"))
              (for _array_element _outactors
                (Class|BPIDialogueEvents|ExecuteDialogueEvent(Message) _array_element (Variables|Default|GetDialogue_CurrentEvent))
                (goto _label)))))))
    (:Is%20Not%20Valid
      (Development|PrintString "Widget Invalid"))))

(event Custom|EV_DialogueCheckContinue
  (bind _dialogue_delayafter (Variables|Default|GetDialogue_DelayAfter))
  (if (Variables|Default|GetDialogue_DelayTimeFinished)
    (Default|ClearDialogue() (Variables|Default|GetDialogue_SubtitleWidget))
    (if (> _dialogue_delayafter 0.0)
      (bind _returnvalue (Utilities|Time|SetTimerbyEvent (delegate Custom|EV_DelayAfterFinished) _dialogue_delayafter))
      (Variables|Default|SetDialogue_TimerDelayAfter _returnvalue)
      (else
        (bind _result (Math|Integer|IncrementInt (Variables|Default|GetDialogue_CurrentDialogueIndex))
          (:%20%20
            (Variables|Default|SetDialogue_CurrentDialogueIndex _result)
            (CallFunction|DialogueNextDialogue)))))))

(event Custom|EV_TimerFinished
  (Variables|Default|SetDialogue_DelayTimeFinished true)
  (switch Utilities|FlowControl|Switch|SwitchonE_DialogueType (Variables|Default|GetDialogue_CurrentLineType)
    (:NewEnumerator0
      (CallFunction|EVDialogueCheckContinue :!label _label))
    (:NewEnumerator4
      (Variables|Default|SetDialogue_State "NewEnumerator2"))
    (:NewEnumerator2
      (bind _outactors (Actor|GetAllActorswithInterface "/Game/DialogueSystem/Blueprints/Interfaces/BPI_DialogueEvents.BPI_DialogueEvents_C"))
      (for _array_element _outactors
        (Class|BPIDialogueEvents|ExecuteDialogueEvent(Message) _array_element (Variables|Default|GetDialogue_CurrentEvent))
        (goto _label)))))

(event Custom|EV_DelayAfterFinished
  (bind _result (Math|Integer|IncrementInt (Variables|Default|GetDialogue_CurrentDialogueIndex))
    (:%20%20
      (Variables|Default|SetDialogue_CurrentDialogueIndex _result)
      (CallFunction|DialogueNextDialogue))))

(event EventInit)

(event EventDialogueContinueConversation
  (CallFunction|DialogueContinueConversation))

(fn DialoguePlayConversation
  (params (Conversation :type Data%20Table%20Object%20Reference))
  (bind _dialogue_subtitlewidget (Variables|Default|GetDialogue_SubtitleWidget))
  (Variables|Default|SetDialogue_CurrentConversation Conversation)
  (CallFunction|ConversationStarted)
  (Variables|Default|SetDialogue_State "NewEnumerator1")
  (Variables|Default|SetDialogue_CurrentDialogueIndex 0)
  (Utilities|IsValid _dialogue_subtitlewidget
    (:Is%20Valid
      (Widget|SetVisibility _dialogue_subtitlewidget "Visible")
      (CallFunction|DialogueLoadConversation (Variables|Default|GetDialogue_CurrentConversation))
      (CallFunction|DialogueNextDialogue))))

(fn DialogueLoadConversation
  (params (Conversation :type Data%20Table%20Object%20Reference))
  (Utilities|Array|Clear (Variables|Default|GetDialogue_Rows))
  (bind _outrownames (DataTable|GetDataTableRowNames Conversation))
  (for _array_element _outrownames
    (bind _returnvalue (Utilities|GetDataTableRow Conversation _array_element)
      (:then
        (Utilities|Array|Add (Variables|Default|GetDialogue_Rows) _returnvalue))))
  (CallFunction|DialogueShowCurrentDialogue))

(fn DialogueShowCurrentDialogue
  (bind _dialogue_rows (Variables|Default|GetDialogue_Rows))
  (bind _dialogue_currentdialogueindex (Variables|Default|GetDialogue_CurrentDialogueIndex))
  (bind _output (Utilities|Array|Get(acopy) _dialogue_rows _dialogue_currentdialogueindex))
  (bind (_order _displaytype _type _speaker _dialogue _duration _delayafter _triggerevent _prompttext) (Utilities|Struct|BreakST_DialogueLine _output))
  (Utilities|IsValid (Variables|Default|GetDialogue_SubtitleWidget)
    (:Is%20Valid
      (CallFunction|DialogueEVShowCurrentDialogueInitVariables _displaytype _type _delayafter _triggerevent)
      (CallFunction|EVShowCurrentDialogue _speaker _dialogue _duration _prompttext))
    (:Is%20Not%20Valid
      (Development|PrintString "Widget INVALID"))))

(fn DialogueEVShowCurrentDialogueInitVariables
  (params (DisplayType :type E_DialogueDisplayType%20Enum :default "NewEnumerator0") (Type :type E_DialogueType%20Enum :default "NewEnumerator0") (DelayAfter :type Float%20%28double-precision%29) (Event :type Name))
  (CallFunction|DialogueUpdateActiveWidget DisplayType)
  (Variables|Default|SetDialogue_CurrentLineType Type)
  (Variables|Default|SetDialogue_DelayTimeFinished false)
  (Variables|Default|SetDialogue_DelayAfter DelayAfter)
  (Variables|Default|SetDialogue_CurrentEvent Event))

(fn DialogueCreateWidget
  (bind _returnvalue (Game|GetPlayerController 0))
  (Utilities|IsValid _returnvalue
    (:Is%20Valid
      (bind _returnvalue_2 (UserInterface|CreateWidget "/Game/DialogueSystem/Blueprints/UI/WBP_Subtitles.WBP_Subtitles_C" _returnvalue))
      (bind _output_get (Variables|Default|SetDialogue_SubtitleWidget _returnvalue_2))
      (UserInterface|Viewport|AddtoViewport _output_get 0))
    (:Is%20Not%20Valid
      (Development|PrintString "NO PLAYER CONTROLLER"))))

(fn DialogueNextDialogue
  (if (< (Variables|Default|GetDialogue_CurrentDialogueIndex) (Utilities|Array|Length (Variables|Default|GetDialogue_Rows)))
    (CallFunction|DialogueShowCurrentDialogue)
    (else
      (CallFunction|DialogueStopConversation))))

(fn DialogueStopConversation
  (bind _dialogue_subtitlewidget (Variables|Default|GetDialogue_SubtitleWidget))
  (Variables|Default|SetDialogue_State "NewEnumerator3")
  (CallFunction|ConversationFinished)
  (Variables|Default|SetDialogue_CurrentDialogueIndex 0)
  (Variables|Default|SetDialogue_CurrentConversation 0)
  (Utilities|Array|Clear (Variables|Default|GetDialogue_Rows))
  (Utilities|IsValid _dialogue_subtitlewidget
    (:Is%20Valid
      (Widget|SetVisibility _dialogue_subtitlewidget "Collapsed")
      (Variables|Default|SetDialogue_State "NewEnumerator0"))))

(fn DialogueContinueConversation
  (if (Utilities|Enum|Equal(Enum) (Variables|Default|GetDialogue_State) "NewEnumerator2")
    (bind _result (Math|Integer|IncrementInt (Variables|Default|GetDialogue_CurrentDialogueIndex))
      (:%20%20
        (Variables|Default|SetDialogue_CurrentDialogueIndex _result)
        (Variables|Default|SetDialogue_State "NewEnumerator1")
        (CallFunction|DialogueNextDialogue)))))

(fn DialogueUpdateActiveWidget
  (params (DisplayType%20 :type E_DialogueDisplayType%20Enum :default "NewEnumerator0"))
  (bind _dialogue_subtitlewidget (Variables|Default|GetDialogue_SubtitleWidget))
  (switch Utilities|FlowControl|Switch|SwitchonE_DialogueDisplayType DisplayType%20
    (:NewEnumerator0
      (Variables|Default|SetDialogue_CurrentWidget _dialogue_subtitlewidget)
      (Widget|SetVisibility _dialogue_subtitlewidget "Visible"))))