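; BP_DialogueComponent drives step-by-step dialogue, advancing each time Interact is called.
; The first call creates WBP_Dialogue with the speaker name and line; later calls update that widget's text.
; Each row from DataTable_2 supplies the next row name, an end flag and a table stored in DataTable, though lookups keep reading DataTable_2.
; Once the end flag is set, the next Interact removes the widget and clears the flag.
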(event EventInteract
  (params (PlayerReference :type BP%20First%20Person%20Character%20ME%20Object%20Reference))
  (if (Variables|Default|GetEndDialouge)
    (Widget|RemovefromParent (Variables|Default|GetActiveDialogueWidget))
    (Variables|Default|SetEndDialouge false)
    (Variables|Default|SetActiveDialogueWidget 0)
    (else
      (Utilities|IsValid (Variables|Default|GetActiveDialogueWidget)
        (:Is%20Valid
          (bind _returnvalue (Utilities|GetDataTableRow "/Game/MYDIALOUGE/DataTable_2.DataTable_2" (Variables|Default|GetRow%20Name))
            (:then
              (Default|UpdateDialouge (Variables|Default|GetActiveDialogueWidget) (.Dialouge (Utilities|Struct|BreakDialogue_Structure _returnvalue)))
              (Variables|Default|SetRow%20Name (.Row (Utilities|Struct|BreakDialogue_Structure _returnvalue)))
              (Variables|Default|SetData%20Table (.Datatable (Utilities|Struct|BreakDialogue_Structure _returnvalue)))
              (Variables|Default|SetEndDialouge (.EndDialogue (Utilities|Struct|BreakDialogue_Structure _returnvalue))))))
        (:Is%20Not%20Valid
          (bind _returnvalue_2 (Utilities|GetDataTableRow "/Game/MYDIALOUGE/DataTable_2.DataTable_2" (Variables|Default|GetRow%20Name))
            (:then
              (bind _returnvalue_3 (UserInterface|CreateWidget "/Game/MYDIALOUGE/WBP_Dialogue.WBP_Dialogue_C" 0 (Utilities|Text|ToText(Name) (Variables|Default|GetSpeakerName)) (.Dialouge (Utilities|Struct|BreakDialogue_Structure _returnvalue_2))))
              (bind _output_get (Variables|Default|SetActiveDialogueWidget _returnvalue_3))
              (UserInterface|Viewport|AddtoViewport _output_get 0)
              (Variables|Default|SetRow%20Name (.Row (Utilities|Struct|BreakDialogue_Structure _returnvalue_2)))
              (Variables|Default|SetData%20Table (.Datatable (Utilities|Struct|BreakDialogue_Structure _returnvalue_2)))
              (Variables|Default|SetEndDialouge (.EndDialogue (Utilities|Struct|BreakDialogue_Structure _returnvalue_2))))))))))