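; BP_DoorCon is an interactive door that swings open when its Interact event fires and HasKey is true.
; A first-person character overlapping DoorCon enables the door's input, while leaving the separate Box component calls DisableInput on the player controller.
; A timeline lerps DoorCon's relative yaw to the open angle, with no closing logic.
; The character's own HasKey is fetched but unused.
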(event OnComponentBeginOverlap(DoorCon)
  (params (OverlappedComponent :type Primitive%20Component%20Object%20Reference) (OtherActor :type Actor%20Object%20Reference) (OtherComp :type Primitive%20Component%20Object%20Reference) (OtherBodyIndex :type Integer) (bFromSweep :type Boolean) (SweepResult :type Hit%20Result%20Structure%20%28by%20ref%29))
  (bind _asbp_first_person_character (Utilities|Casting|CastToBP_FirstPersonCharacterME OtherActor))
  (Input|EnableInput (Game|GetPlayerController 0)))

(event OnComponentEndOverlap(Box)
  (params (OverlappedComponent :type Primitive%20Component%20Object%20Reference) (OtherActor :type Actor%20Object%20Reference) (OtherComp :type Primitive%20Component%20Object%20Reference) (OtherBodyIndex :type Integer))
  (Utilities|Casting|CastToBP_FirstPersonCharacterME OtherActor)
  (Input|DisableInput (Game|GetPlayerController 0) 0))

(event EventBeginPlay)

(event Collision|EventActorBeginOverlap
  (params (OtherActor :type Actor%20Object%20Reference)))

(event EventTick
  (params (DeltaSeconds :type Float%20%28single-precision%29)))

(event EventInteract
  (if (Variables|Default|GetHasKey?)
    (bind _newtrack_0 (Timeline|Timeline Play)
      (:Update
        (Transformation|SetRelativeRotation (Variables|Default|GetDoorCon) (Math|Rotator|MakeRotator 0.0 0.0 (Math|Float|Lerp 0.0 -1.2e+02 _newtrack_0)) false false)))))

(fn ConstructionScript)