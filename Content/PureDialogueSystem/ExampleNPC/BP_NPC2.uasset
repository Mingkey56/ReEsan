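; Example talkable NPC for the Pure Dialogue System that offers a "Talk" interaction prompt.
; Interacting stores the interactor and starts the dialog on its dialog component.
; The component's "Push" trigger event ends the dialog and launches the interacting character backwards, opposite to its facing direction.
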(event TriggerEvent(BP_DialogComponent)
  (params (Trigger :type E_DialogTriggers%20Enum :default "NewEnumerator0"))
  (switch Utilities|FlowControl|Switch|SwitchonE_DialogTriggers Trigger
    (:NewEnumerator2
      (Default|EndDialog (Variables|Default|GetBP_DialogComponent))
      (bind _ascharacter (Utilities|Casting|CastToCharacter (Variables|Default|GetInteractor)))
      (Character|LaunchCharacter _ascharacter (* (Math|Vector|Normalize (* (Transformation|GetActorForwardVector (Variables|Default|GetInteractor)) -1.0)) 2e+03) false false))))

(event EventBeginPlay)

(event Collision|EventActorBeginOverlap
  (params (OtherActor :type Actor%20Object%20Reference)))

(event EventTick
  (params (DeltaSeconds :type Float%20%28single-precision%29)))

(event EventInteract
  (params (Interactor :type Actor%20Object%20Reference))
  (Variables|Default|SetInteractor Interactor)
  (Default|StartDialog (Variables|Default|GetBP_DialogComponent)))

(fn ConstructionScript)

(fn GetInteractionText
  (return "Talk"))