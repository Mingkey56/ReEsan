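; BP_BIS_Door is a door actor in the Basic Interaction System that swings open and closed through interface interactions.
; An Open request needs IsUnlocked, while an Unlock request skips that check, and both require CanOpen.
; A FlipFlop alternates a Timeline forward and in reverse to drive the actor's yaw.
; CanOpen blocks retriggering during motion and resets shortly after the Timeline finishes.
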(event Custom|Event%20Rotate%20Door
  ;[0.4118 0.9216 1] Event Rotate Door
  (Utilities|FlowControl|FlipFlop
    (:A
      (bind _angle (Timeline|Timeline Play)
        (:Update
          (Variables|Default|SetCan%20Open? false)
          (Transformation|SetActorRotation (Math|Rotator|MakeRotator 0.0 0.0 _angle)))
        (:Finished
          (Utilities|FlowControl|Delay 0.2)
          (Variables|Default|SetCan%20Open? true))))
    (:B
      (Timeline|Timeline ReverseFromEnd))))

(event EventUpdateInteract
  (params (Actor :type Actor%20Object%20Reference) (Status :type E_BIS_ItemType%20Enum :default "NewEnumerator0") (Widget :type WBP%20BIS%20Inventory%20Object%20Reference))
  ;[1 1 0] Event Update Interact (Interface)
  (switch Utilities|FlowControl|Switch|SwitchonE_BIS_ItemType Status
    (:NewEnumerator3
      (if (Variables|Default|GetIs%20Unlocked?)
        (if (Variables|Default|GetCan%20Open?) :!label _label
          (CallFunction|EventRotateDoor))))
    (:NewEnumerator5
      (goto _label))))

(fn ConstructionScript)